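; BP_Enemy is a basic enemy that endlessly chases the first player character and can be killed by damage.
; Any damage is subtracted from EnemyHealth, and the actor destroys itself once health runs out.
; On BeginPlay it starts AI Move To toward the player, with further Move To nodes looping into each other on success or failure, without a behavior tree or attack logic.
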(event EventBeginPlay
  ;[0.15 0.15 0.15 0.5] Enemy AI
  (AI|AIMoveTo self "0, 0, 0" (Game|GetPlayerCharacter 0) 1e+02 false
    (:OnSuccess
      (AI|AIMoveTo self "0, 0, 0" (Game|GetPlayerCharacter 0) 5.0 false :!label _label
        (:OnSuccess
          _)
        (:OnFail
          _))
      (AI|AIMoveTo self "0, 0, 0" (Game|GetPlayerCharacter 0) 5.0 false :!label _label_2
        (:OnSuccess
          (goto _label))
        (:OnFail
          (goto _label))))
    (:OnFail
      (goto _label_2))))

(event Game|Damage|EventAnyDamage
  (params (Damage :type Float%20%28single-precision%29) (DamageType :type Damage%20Type%20Object%20Reference) (InstigatedBy :type Controller%20Object%20Reference) (DamageCauser :type Actor%20Object%20Reference))
  ;[0.15 0.15 0.15 0.5] Enemy Health
  (Variables|Default|SetEnemyHealth (- (Variables|Default|GetEnemyHealth) Damage))
  (if (<= (Variables|Default|GetEnemyHealth) 0.0)
    (Actor|DestroyActor)))

(fn ConstructionScript)